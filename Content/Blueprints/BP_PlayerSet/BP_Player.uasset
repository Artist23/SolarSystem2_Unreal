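; BP_Player is a gaze-controlled player with a 3D cursor for interacting with BP_Quiz and BP_Dashboard actors.
; Every tick a camera line trace shows the cursor just before the hit, scaled by distance, or hides it otherwise.
; While on target, WidgetInteraction presses the left mouse key and releases it after a one-second delay or on Pull Trigger.
; Turn and LookUp axes emulate head rotation.
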(event Custom|Gaze%20Check
  (bind _camera (Variables|Default|GetCamera))
  (bind _cursor (Variables|Default|GetCursor))
  (bind _camera_2 (Variables|Default|GetCamera))
  (bind _returnvalue (Transformation|GetWorldLocation _camera))
  ;[1 1 1] Gaze Check
  (bind _outhit (Collision|LineTraceByChannel _returnvalue (+ (* (Math|Vector|GetForwardVector _camera) 1e+06) _returnvalue) "TraceTypeQuery1" false 0 "None" true "(R=0.950615,G=0.921184,B=1.000000,A=1.000000)"))
  (Utilities|FlowControl|Sequence
    (:then_0
      ;[1 1 1] Hit Test
      (if (or (== (Utilities|GetClass (.HitActor (Collision|BreakHitResult _outhit))) "/Game/Blueprints/BP_Quiz.BP_Quiz_C") (== (Utilities|GetClass (.HitActor (Collision|BreakHitResult _outhit))) "/Game/Blueprints/BP_PlayerSet/BP_Dashboard.BP_Dashboard_C"))
        (Utilities|FlowControl|Sequence
          (:then_0
            ;[1 1 1] Set cursor's position and scale
            (CallFunction|ActivateCusor)
            (bind _output_get (Variables|Default|SetHitDistance (.Distance (Collision|BreakHitResult _outhit))))
            (Utilities|FlowControl|Sequence
              (:then_0
                (Transformation|SetWorldScale3D _cursor (* (Variables|Default|GetOriginalScaleCursor) (* _output_get 0.007))))
              (:then_1
                (Transformation|SetWorldLocation _cursor (+ (Transformation|GetWorldLocation _camera_2) (* (Math|Vector|GetForwardVector _camera_2) (* _output_get 0.95))) false false))))
          (:then_1
            ;[1 1 1] Button Click
            (Class|WidgetInteractionComponent|PressPointerKey (Variables|Default|GetWidgetInteraction) "LeftMouseButton")
            (Utilities|FlowControl|Delay 1.0)
            (Class|WidgetInteractionComponent|ReleasePointerKey (Variables|Default|GetWidgetInteraction) "LeftMouseButton")))
        (else
          (CallFunction|DeactivateCursor))))))

(event EventTick
  (params (DeltaSeconds :type Float%20%28single-precision%29))
  (CallFunction|GazeCheck))

(event EventBeginPlay
  ;[1 1 1] Get the original scale
  (Variables|Default|SetOriginalScaleCursor (Transformation|GetWorldScale (Variables|Default|GetCursor))))

(event Input|ActionEvents|InputActionPullTrigger
  (params (Key :type Key%20Structure))
  (:Pressed
    ;[1 1 1] Button Click
    (Class|WidgetInteractionComponent|ReleasePointerKey (Variables|Default|GetWidgetInteraction) "LeftMouseButton")))

(event Input|AxisEvents|InputAxisTurn
  (params (AxisValue :type Float%20%28single-precision%29))
  ;[1 1 1] Emulator
  (Pawn|Input|AddControllerYawInput AxisValue))

(event Input|AxisEvents|InputAxisLookUp
  (params (AxisValue :type Float%20%28single-precision%29))
  ;[1 1 1] Emulator
  (Pawn|Input|AddControllerPitchInput AxisValue))

(fn ConstructionScript)

(fn ActivateCusor
  (Rendering|SetVisibility (Variables|Default|GetCursor) true false))

(fn DeactivateCursor
  (Rendering|SetVisibility (Variables|Default|GetCursor) false false))